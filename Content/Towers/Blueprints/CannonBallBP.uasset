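; Cannonball projectile for towers that damages BasicMonsters by direct hit and expanding splash, configured through SetDefaults.
; Tick moves it forward with a hand-rolled drop that grows each frame, until it hits a monster or a fixed ground height.
; It then shows a randomly chosen, rotated explosion mesh, scaled up in timed steps until it reaches Size and the actor is destroyed.
; Overlaps during the explosion deal splash once per monster, tracked in ImmuneMonsters.
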(event Collision|EventActorBeginOverlap
  (params (OtherActor :type Actor%20Object%20Reference))
  (bind _cannonball_explosion (Variables|Default|GetCannonBall/Explosion))
  (bind _asbasic_monster (Utilities|Casting|CastToBasicMonster OtherActor))
  (if (Variables|Default|GetExploding)
    (bind _new (CallFunction|DealSplash _asbasic_monster))
    (if _new
      (Default|TakeDamage _asbasic_monster (Variables|Default|GetSplashDamage)))
    (else
      (Default|TakeDamage _asbasic_monster (Variables|Default|GetDirectDamage))
      (Variables|Default|SetExploding true)
      (Components|StaticMesh|SetStaticMesh _cannonball_explosion (Utilities|Select :Index (Math|Random|RandomInteger 3) :Option%200 "/Game/Towers/Blueprints/ProjectileMeshes/Explosion1.Explosion1" :Option%201 "/Game/Towers/Blueprints/ProjectileMeshes/Explosion2.Explosion2" :Option%202 "/Game/Towers/Blueprints/ProjectileMeshes/Explosion3.Explosion3"))
      (Transformation|SetWorldRotation _cannonball_explosion (Math|Rotator|MakeRotator (Math|Random|RandomFloatinRange 0.0 3.6e+02) (Math|Random|RandomFloatinRange 0.0 3.6e+02) (Math|Random|RandomFloatinRange 0.0 3.6e+02)) false false)
      (bind _output_get (Variables|Default|SetCurrentScale "0.500000,0.500000,0.500000"))
      (Transformation|SetWorldScale3D _cannonball_explosion _output_get)
      (Utilities|FlowControl|Delay 0.1 :!label _label)
      (bind _output_get_2 (Variables|Default|SetCurrentScale (* _output_get (+ (/ (Variables|Default|GetSize) 21.700001) 1.0))))
      (Transformation|SetWorldScale3D _cannonball_explosion _output_get_2)
      (if (>= (.x (Variables|Default|GetCurrentScale)) (Variables|Default|GetSize))
        (Actor|DestroyActor)
        (else
          (goto _label))))))

(event EventTick
  (params (DeltaSeconds :type Float%20%28single-precision%29))
  (bind _cannonball_explosion (Variables|Default|GetCannonBall/Explosion))
  (bind _base (Variables|Default|GetBase))
  (bind _speed (Variables|Default|GetSpeed))
  (bind _returnvalue (Math|Vector|GetForwardVector _base))
  (bind _returnvalue_2 (* DeltaSeconds _speed 64.127998))
  (bind _returnvalue_3 (* _returnvalue _returnvalue_2))
  (if (not (Variables|Default|GetExploding))
    (Transformation|SetWorldLocation _base (+ (Math|Vector|MakeVector (.x _returnvalue_3) (.y _returnvalue_3) (* (* (Variables|Default|GetDown) DeltaSeconds) -2.2)) (Transformation|GetWorldLocation _base)) false false)
    (Math|Integer|IncrementInt (Variables|Default|GetDown)
      (:%20%20
        (if (<= (.z (Transformation|GetWorldLocation _base)) 2e+02)
          (Variables|Default|SetExploding true)
          (Components|StaticMesh|SetStaticMesh _cannonball_explosion (Utilities|Select :Index (Math|Random|RandomInteger 3) :Option%200 "/Game/Towers/Blueprints/ProjectileMeshes/Explosion1.Explosion1" :Option%201 "/Game/Towers/Blueprints/ProjectileMeshes/Explosion2.Explosion2" :Option%202 "/Game/Towers/Blueprints/ProjectileMeshes/Explosion3.Explosion3"))
          (Transformation|SetWorldRotation _cannonball_explosion (Math|Rotator|MakeRotator (Math|Random|RandomFloatinRange 0.0 3.6e+02) (Math|Random|RandomFloatinRange 0.0 3.6e+02) (Math|Random|RandomFloatinRange 0.0 3.6e+02)) false false)
          (bind _output_get (Variables|Default|SetCurrentScale "0.500000,0.500000,0.500000"))
          (Transformation|SetWorldScale3D _cannonball_explosion _output_get)
          (Utilities|FlowControl|Delay 0.1 :!label _label)
          (bind _output_get_2 (Variables|Default|SetCurrentScale (* _output_get (+ (/ (Variables|Default|GetSize) 21.700001) 1.0))))
          (Transformation|SetWorldScale3D _cannonball_explosion _output_get_2)
          (if (>= (.x (Variables|Default|GetCurrentScale)) (Variables|Default|GetSize))
            (Actor|DestroyActor)
            (else
              (goto _label))))))))

(event EventBeginPlay
  (Variables|Default|SetExploding false)
  (Variables|Default|SetDown 1))

(fn ConstructionScript)

(fn SetDefaults
  (params (Direct :type Integer) (Splash :type Integer) (Speed :type Float%20%28single-precision%29) (ExplosionSize :type Float%20%28single-precision%29))
  (Variables|Default|SetDirectDamage Direct)
  (Variables|Default|SetSplashDamage Splash)
  (Variables|Default|SetSpeed Speed)
  (Variables|Default|SetSize ExplosionSize))

(fn DealSplash
  (params (NewMonster :type Basic%20Monster%20Object%20Reference))
  (bind _output_get (LocalVariables|SetFound false))
  (for _array_element (Variables|Default|GetImmuneMonsters)
    (LocalVariables|SetFound (or (== _array_element NewMonster) _output_get)))
  (if _output_get
    (return false)
    (else
      (Utilities|Array|Add (Variables|Default|GetImmuneMonsters) NewMonster)
      (return true))))