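; MagicShot is a homing tower projectile that damages and slows monsters.
; Each tick it turns toward its target Monster, if valid, and moves its Magic component forward at a scaled Speed.
; Overlapping the target applies full damage and slow, then destroys the shot, while other BasicMonsters take weakened effects and let it pass.
; It also destroys itself when Magic drops below world height zero.
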(event Collision|EventActorBeginOverlap
  (params (OtherActor :type Actor%20Object%20Reference))
  (bind _monster (Variables|Default|GetMonster))
  (bind _damage (Variables|Default|GetDamage))
  (bind _slow (Variables|Default|GetSlow))
  (bind _duration (Variables|Default|GetDuration))
  (bind _asbasic_monster (Utilities|Casting|CastToBasicMonster OtherActor))
  (if (== _asbasic_monster _monster)
    (Default|TakeDamage _monster _damage)
    (Default|Slow _monster _slow _duration)
    (Actor|DestroyActor)
    (else
      (Default|TakeDamage _asbasic_monster (/ _damage 2))
      (Default|Slow _asbasic_monster (/ _slow 2.5) (/ _duration 2.5)))))

(event EventTick
  (params (DeltaSeconds :type Float%20%28single-precision%29))
  (bind _magic (Variables|Default|GetMagic))
  (bind _magic_2 (Variables|Default|GetMagic))
  (Utilities|IsValid (Variables|Default|GetMonster)
    (:Is%20Valid
      (CallFunction|TurntoTarget))
    (:Is%20Not%20Valid
      _))
  (Transformation|SetWorldLocation _magic (+ (* (Math|Vector|GetForwardVector _magic) (* DeltaSeconds (Variables|Default|GetSpeed) 21.700001)) (Transformation|GetWorldLocation _magic)) false false)
  (Utilities|IsValid _magic_2
    (:Is%20Valid
      (if (< (.z (Transformation|GetWorldLocation _magic_2)) 0.0)
        (Actor|DestroyActor)))))

(fn ConstructionScript)

(fn TurntoTarget
  (Transformation|SetActorRotation (Math|Rotator|FindLookatRotation (Transformation|GetActorLocation) (Transformation|GetActorLocation (Variables|Default|GetMonster)))))