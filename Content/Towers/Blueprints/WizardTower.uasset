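; WizardTower is a tower Blueprint that fires MagicShot projectiles at monsters.
; LevelUp calls the parent, then, unless it returned true or Level is 1, selects range, reload, shot speed, damage and slow stats by level.
; FireAt, gated by ShotDelay, spawns a scaled-up shot above the tower aimed at the monster's mesh and passes it the target, speed and damage, but no slow values.
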(event EventBeginPlay
  (|CallParentFunction) ; This node is disabled and will not be called.\nDrag off pins to build functionality.
)

(event Collision|EventActorBeginOverlap
  (params (OtherActor :type Actor%20Object%20Reference))
  (|CallParentFunction OtherActor) ; This node is disabled and will not be called.\nDrag off pins to build functionality.
)

(event EventTick
  (params (DeltaSeconds :type Float%20%28single-precision%29))
  (|CallParentFunction DeltaSeconds) ; This node is disabled and will not be called.\nDrag off pins to build functionality.
)

(fn ConstructionScript
  (|CallParentFunction))

(fn LevelUp
  (bind _level (Variables|Default|GetLevel))
  (bind _returnvalue (- _level 2))
  (bind _alreadymaxed (|CallParentFunction))
  (if (or _alreadymaxed (== (Variables|Default|GetLevel) 1))
    (return _alreadymaxed)
    (else
      (Utilities|FlowControl|Sequence
        (:then_0
          (Variables|Default|SetRange (Utilities|Select :Index _returnvalue :Option%200 4321.0 :Option%201 4444.0 :Option%202 4567.0))
          (Variables|Default|SetReloadTime (Utilities|Select :Index _returnvalue :Option%200 9.9 :Option%201 8.7 :Option%202 7.0))
          (Variables|Default|SetShotSpeed (Utilities|Select :Index _returnvalue :Option%200 21.700001 :Option%201 21.700001 :Option%202 64.127998))
          (Variables|Default|SetDamage (Utilities|Select :Index _returnvalue :Option%200 42 :Option%201 55 :Option%202 59))
          (Variables|Default|SetSlowPercent (Utilities|Select :Index _returnvalue :Option%200 0.9 :Option%201 0.85 :Option%202 0.77))
          (Variables|Default|SetSlowDuration (Utilities|Select :Index _returnvalue :Option%200 2.8 :Option%201 3.0 :Option%202 3.33)))
        (:then_1
          (return _alreadymaxed))))))

(fn Fireat
  (params (Monster :type Basic%20Monster%20Object%20Reference))
  (bind _tower (Variables|Default|GetTower))
  (bind _mesh (Variables|/Script/Engine.Character|GetMesh Monster))
  (bind _returnvalue (Transformation|GetWorldLocation _tower))
  (bind _returnvalue_2 (+ (.z _returnvalue) 999.0))
  (if (<= (Variables|Default|GetShotDelay) 0.0)
    (Variables|Default|SetShotDelay (Variables|Default|GetReloadTime))
    (bind _returnvalue_3 (Game|SpawnActorfromClass "/Game/Towers/Blueprints/MagicShot.MagicShot_C" (Math|Transform|MakeTransform (Math|Vector|MakeVector (.x _returnvalue) (.y _returnvalue) _returnvalue_2) (Math|Rotator|FindLookatRotation (Math|Vector|MakeVector (.x _returnvalue) (.y _returnvalue) _returnvalue_2) (+ (Transformation|GetWorldLocation _mesh) (Math|Vector|GetRightVector _mesh))) "7.000000,7.000000,7.000000") "Undefined" 0 0))
    (Variables|/Game/Towers/Blueprints/MagicShot.MagicShot_C|SetMonster _returnvalue_3 Monster)
    (Variables|/Game/Towers/Blueprints/MagicShot.MagicShot_C|SetSpeed _returnvalue_3 (Variables|Default|GetShotSpeed))
    (Variables|/Game/Towers/Blueprints/MagicShot.MagicShot_C|SetDamage _returnvalue_3 (Variables|Default|GetDamage))))