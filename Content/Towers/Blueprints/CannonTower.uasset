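; Cannon tower Blueprint for a tower defense game that shoots cannonballs at monsters and can level up.
; FireAt, gated by ShotDelay, spawns a CannonBallBP above the tower aimed at the monster's mesh and passes it damage, speed and level-scaled splash and explosion size.
; LevelUp calls the parent, then boosts range, fire rate, shot speed and damage unless the parent returns true or Level is 1.
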(event EventBeginPlay
  (|CallParentFunction) ; This node is disabled and will not be called.\nDrag off pins to build functionality.
)

(event Collision|EventActorBeginOverlap
  (params (OtherActor :type Actor%20Object%20Reference))
  (|CallParentFunction OtherActor) ; This node is disabled and will not be called.\nDrag off pins to build functionality.
)

(event EventTick
  (params (DeltaSeconds :type Float%20%28single-precision%29))
  (|CallParentFunction DeltaSeconds))

(fn ConstructionScript
  (|CallParentFunction))

(fn Fireat
  (params (Monster :type Basic%20Monster%20Object%20Reference))
  (bind _tower (Variables|Default|GetTower))
  (bind _mesh (Variables|/Script/Engine.Character|GetMesh Monster))
  (bind _damage (Variables|Default|GetDamage))
  (bind _level (Variables|Default|GetLevel))
  (bind _returnvalue (Transformation|GetWorldLocation _tower))
  (bind _returnvalue_2 (+ (.z _returnvalue) 6e+02))
  (if (<= (Variables|Default|GetShotDelay) 0.0)
    (Variables|Default|SetShotDelay (Variables|Default|GetReloadTime))
    (bind _returnvalue_3 (Game|SpawnActorfromClass "/Game/Towers/Blueprints/CannonBallBP.CannonBallBP_C" (Math|Transform|MakeTransform (Math|Vector|MakeVector (.x _returnvalue) (.y _returnvalue) _returnvalue_2) (Math|Rotator|FindLookatRotation (Math|Vector|MakeVector (.x _returnvalue) (.y _returnvalue) _returnvalue_2) (+ (Transformation|GetWorldLocation _mesh) (Math|Vector|GetRightVector _mesh))) "1,1,1") "Undefined" 0 0))
    (Default|SetDefaults _returnvalue_3 _damage (/ _damage (- 6 _level)) (Variables|Default|GetShotSpeed) (* _level 6.0))))

(fn LevelUp
  (bind _alreadymaxed (|CallParentFunction))
  (if (or _alreadymaxed (== (Variables|Default|GetLevel) 1))
    (return _alreadymaxed)
    (else
      (Utilities|FlowControl|Sequence
        (:then_0
          (Variables|Default|SetRange (* (Variables|Default|GetRange) 1.234567))
          (Variables|Default|SetReloadTime (/ (Variables|Default|GetReloadTime) 1.234567))
          (Variables|Default|SetShotSpeed (+ (Variables|Default|GetShotSpeed) 2.2))
          (Variables|Default|SetDamage (+ (Variables|Default|GetDamage) 3)))
        (:then_1
          (return _alreadymaxed))))))