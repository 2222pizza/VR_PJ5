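; Arrow projectile for towers that damages monsters it hits.
; GO sets damage and speed and starts flight, which Tick advances through ServerTick along the forward vector without sweeping, destroying the arrow at or below world Z zero.
; Overlap with a BasicMonster, handled in ServerOverlap, applies damage, ends flight and attaches the arrow to the monster, keeping its world position and rotation so it stays stuck.
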(event Custom|ServerTick
  (params (Delta%20Seconds :type Float%20%28single-precision%29))
  (bind _base (Variables|Default|GetBase))
  (if (Variables|Default|GetFlying)
    (Transformation|SetWorldLocation _base (+ (* (Math|Vector|GetForwardVector _base) (* Delta%20Seconds (* (Variables|Default|GetArrowSpeed) 721.0))) (Transformation|GetWorldLocation _base)) false false)
    (if (<= (.z (Transformation|GetWorldLocation _base)) 0.0)
      (Actor|DestroyActor))))

(event Custom|ServerOverlap
  (params (Other%20Actor :type Actor%20Object%20Reference))
  (if (Variables|Default|GetFlying)
    (bind _asbasic_monster (Utilities|Casting|CastToBasicMonster Other%20Actor))
    (Variables|Default|SetFlying false)
    (Default|TakeDamage _asbasic_monster (Variables|Default|GetDamage))
    (Transformation|AttachActorToActor _asbasic_monster "None" "KeepWorld" "KeepWorld" "KeepRelative" false)))

(event Collision|EventActorBeginOverlap
  (params (OtherActor :type Actor%20Object%20Reference))
  (CallFunction|ServerOverlap OtherActor))

(event EventTick
  (params (DeltaSeconds :type Float%20%28single-precision%29))
  (CallFunction|ServerTick DeltaSeconds))

(fn ConstructionScript)

(fn GO
  (params (Damage :type Integer) (Speed :type Float%20%28single-precision%29))
  (Variables|Default|SetDamage Damage)
  (Variables|Default|SetArrowSpeed Speed)
  (Variables|Default|SetFlying true))