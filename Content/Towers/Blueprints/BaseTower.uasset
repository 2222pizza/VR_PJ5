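; Base tower Blueprint that provides shared range, leveling and shot cooldown logic, with an empty FireAt function that takes a monster.
; Tick passes delta time to ServerTick, which counts ShotDelay down.
; LevelUp swaps to the next mesh in Meshes and updates the level text, returning true only when already maxed.
; The construction script calls LevelUp to apply the initial mesh and label.
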(event Custom|ServerTick
  (params (Delta%20Seconds :type Float%20%28single-precision%29))
  (Variables|Default|SetShotDelay (select (<= (Variables|Default|GetShotDelay) 0.0) 0.0 (- (Variables|Default|GetShotDelay) Delta%20Seconds))))

(event EventTick
  (params (DeltaSeconds :type Float%20%28single-precision%29))
  (CallFunction|ServerTick DeltaSeconds))

(fn ConstructionScript
  (CallFunction|LevelUp))

(fn GetRange
  (return (Variables|Default|GetRange)))

(fn Fireat
  (params (Monster :type Basic%20Monster%20Object%20Reference)))

(fn LevelUp
  (bind _level (Variables|Default|GetLevel))
  (bind _meshes (Variables|Default|GetMeshes))
  (if (>= _level (Utilities|Array|Length _meshes))
    (return true)
    (else
      (Components|StaticMesh|SetStaticMesh (Variables|Default|GetTower) (Utilities|Array|Get(acopy) _meshes _level))
      (Math|Integer|IncrementInt _level
        (:%20%20
          (Rendering|Components|TextRender|SetText (Variables|Default|GetTowerLevelText) (Utilities|Text|ToText(String) (Utilities|String|Append "Level: " (Utilities|String|ToString(Integer) _level))))
          (return false))))))