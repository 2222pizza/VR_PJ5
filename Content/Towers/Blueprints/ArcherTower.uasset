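; Archer tower Blueprint that shoots volleys of TowerArrowBP arrows at monsters.
; FireAt, gated by Shooting and ShotDelay, aims once from above the tower at an offset point on the monster's mesh.
; FireArrows loops through Delay to launch one arrow per Level along that transform, then starts the reload.
; LevelUp raises range and shot speed and lowers reload time and damage when the parent returns false and Level isn't 1.
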(event Custom|Fire%20Arrows
  (params (Spawn :type Transform))
  (bind _output_get (Variables|Default|SetArrowsLeft (Variables|Default|GetLevel)))
  (bind _returnvalue (Game|SpawnActorfromClass "/Game/Towers/Blueprints/TowerArrowBP.TowerArrowBP_C" Spawn "AlwaysSpawn" 0 0 :!label _label))
  (bind _result (Math|Integer|DecrementInt _output_get)
    (:%20%20
      (Default|GO _returnvalue (Variables|Default|GetDamage) (Variables|Default|GetShotSpeed))
      (if (> _result 0)
        (Utilities|FlowControl|Delay 0.5)
        (goto _label)
        (else
          (Variables|Default|SetShotDelay (Variables|Default|GetReloadTime))
          (Variables|Default|SetShooting false))))))

(event EventBeginPlay
  (|CallParentFunction) ; This node is disabled and will not be called.\nDrag off pins to build functionality.
)

(event Collision|EventActorBeginOverlap
  (params (OtherActor :type Actor%20Object%20Reference))
  (|CallParentFunction OtherActor) ; This node is disabled and will not be called.\nDrag off pins to build functionality.
)

(event EventTick
  (params (DeltaSeconds :type Float%20%28single-precision%29))
  (|CallParentFunction DeltaSeconds))

(fn ConstructionScript
  (|CallParentFunction))

(fn Fireat
  (params (Monster :type Basic%20Monster%20Object%20Reference))
  (bind _tower (Variables|Default|GetTower))
  (bind _mesh (Variables|/Script/Engine.Character|GetMesh Monster))
  (bind _returnvalue (Math|Vector|GetRightVector _mesh))
  (bind _returnvalue_2 (Transformation|GetWorldLocation _tower))
  (bind _returnvalue_3 (Transformation|GetWorldLocation _mesh))
  (bind _returnvalue_4 (* _returnvalue 2.2))
  (bind _returnvalue_5 (+ (.z _returnvalue_2) 5e+02))
  (bind _returnvalue_6 (+ _returnvalue_3 _returnvalue_4))
  (if (and (not (Variables|Default|GetShooting)) (<= (Variables|Default|GetShotDelay) 0.0))
    (Variables|Default|SetShooting true)
    (CallFunction|FireArrows (Math|Transform|MakeTransform (Math|Vector|MakeVector (.x _returnvalue_2) (.y _returnvalue_2) _returnvalue_5) (Math|Rotator|FindLookatRotation (Math|Vector|MakeVector (.x _returnvalue_2) (.y _returnvalue_2) _returnvalue_5) (Math|Vector|MakeVector (.x _returnvalue_6) (.y _returnvalue_6) (+ (.z _returnvalue_6) 55.0))) "1,1,1"))))

(fn LevelUp
  (bind _alreadymaxed (|CallParentFunction))
  (if (or _alreadymaxed (== (Variables|Default|GetLevel) 1))
    (return _alreadymaxed)
    (else
      (Utilities|FlowControl|Sequence
        (:then_0
          (Variables|Default|SetRange (+ (Variables|Default|GetRange) 1e+02))
          (Math|Float|DecrementFloat (Variables|Default|GetReloadTime)
            (:%20%20
              (Variables|Default|SetShotSpeed (* (Variables|Default|GetShotSpeed) 1.5))
              (Math|Integer|DecrementInt (Variables|Default|GetDamage)))))
        (:then_1
          (return _alreadymaxed))))))